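; Lobby player state that holds each player's chosen color and applies it, with the player's name, to their BP_LobbyCharacter pawn.
; A server event sets PlayerColor, whose OnRep handler calls UpdatePlayer to refresh the pawn.
; BeginPlay runs the same update after a fixed two-second delay, and the update does nothing if the pawn cast fails.
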(event `Update Player`
  (bind _asbp_lobby_character (cast `/Game/Blueprints/Characters/BP_LobbyCharacter` (`self.GetPawn`) :!label _label))
  (`/Game/Blueprints/Characters/BP_LobbyCharacter.Set Player Name` _asbp_lobby_character (`self.GetPlayerName`))
  (`/Game/Blueprints/Characters/BP_LobbyCharacter.Set Player Color` _asbp_lobby_character (`self.Player Color`)))

(event `self.ReceiveBeginPlay`
  (`KismetSystemLibrary.Delay` 2.0)
  (goto _label))

(event `SR Set Player Color In Player State`
  (params (`Player Color` :type "/Game/Blueprints/Structures/F_PlayerColor Structure"))
  ;[0 0 0] Set Player Color In Server
  (set `self.Player Color` `Player Color`))

(fn `OnRep_Player Color`
  (`self.Update Player`))

(fn `UserConstructionScript`)