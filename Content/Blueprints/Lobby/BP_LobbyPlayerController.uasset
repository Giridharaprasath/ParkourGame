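; Lobby player controller that routes pause, controls-toggle and interact input, plus get-up and interact hints, to BP_LobbyHUD.
; The interact key opens the player customization UI only when color change is allowed.
; The construction script reads the player color from BP_MyGameInstance.
; OCSetupPlayer waits briefly, then passes that color to BP_LobbyPlayerState through SRSetPlayerColorInPlayerState.
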(event `Show Get Up Hint`
  (params (`Can Get Up` :type Boolean))
  ;[0 0 0] Show Get Up Hint Function
  (bind _output_get (set `self.Can Get Up` `Can Get Up`))
  (`/Game/Blueprints/Lobby/BP_LobbyHUD.Show Get Up Hint` (`self.As BP Lobby HUD`) _output_get))

(event `self.ReceiveBeginPlay`
  (`WidgetBlueprintLibrary.SetInputMode_GameOnly` self)
  (set `self.As BP Lobby HUD` (cast `/Game/Blueprints/Lobby/BP_LobbyHUD` (`self.GetHUD`) :!pure true)))

(event `Show Interact Hint`
  (params (`Can Change Color` :type Boolean))
  ;[0 0 0] Show Interact Hint Function
  (bind _output_get (set `self.Can Change Color` `Can Change Color`))
  (`/Game/Blueprints/Lobby/BP_LobbyHUD.Show Interact Hint` (`self.As BP Lobby HUD`) _output_get))

(event `InputAction|Pause Game`
  (params (Key :type "Key Structure"))
  ;[0 0 0] Pause Game Input Action
  (:`Pressed`
    (`/Game/Blueprints/Lobby/BP_LobbyHUD.Pause Game` (`self.As BP Lobby HUD`))))

(event `InputAction|Toggle Hint`
  (params (Key :type "Key Structure"))
  ;[0 0 0] Toggle Controls Input Action
  (:`Pressed`
    (`/Game/Blueprints/Lobby/BP_LobbyHUD.Toggle Controls` (`self.As BP Lobby HUD`))))

(event `InputAction|Interact`
  (params (Key :type "Key Structure"))
  ;[0 0 0] Open Player Change UI Input Action
  (:`Pressed`
    (if (`self.Can Change Color`)
      (`/Game/Blueprints/Lobby/BP_LobbyHUD.Open Player Change UI` (`self.As BP Lobby HUD`) self)
      (`KismetSystemLibrary.PrintString` "Opening Player Customization"))))

(event `OC Setup Player`
  (`KismetSystemLibrary.Delay` 2.0)
  (`self.Try Player Color` (`self.Player Color`)))

(event `Try Player Color`
  (params (`Player Color` :type "/Game/Blueprints/Structures/F_PlayerColor Structure"))
  ;[0 0 0] Try Player Color Function
  (bind _asbp_lobby_player_state (cast `/Game/Blueprints/Lobby/BP_LobbyPlayerState` (`self.PlayerState`)))
  (`/Game/Blueprints/Lobby/BP_LobbyPlayerState.SR Set Player Color In Player State` _asbp_lobby_player_state `Player Color`))

(fn `Change Camera`)

(fn `Get Player Color From Game Instance`
  (bind _asbp_my_game_instance (cast `/Game/Blueprints/BP_MyGameInstance` (`GameplayStatics.GetGameInstance`)))
  (set `self.Player Color` (`/Game/Blueprints/BP_MyGameInstance.Player Color` _asbp_my_game_instance)))

(fn `UserConstructionScript`
  (`self.Get Player Color From Game Instance`))