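; Lobby HUD that manages the pause menu, help overlay and player color change screen, and draws a player name on screen.
; It creates the pause and help widgets on BeginPlay, with events that show the pause menu, toggle controls and set interact and get-up hints.
; The color change widget is created on first open, takes UI-only input and receives its player image reference from the lobby character.
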(event `self.ReceiveBeginPlay`
  (bind _returnvalue (`self.GetOwningPlayerController`))
  (`WidgetLayoutLibrary.RemoveAllWidgets`)
  (bind _returnvalue_2 (`|CreateWidget` "/Game/UI/PauseMenu/WBP_PauseMenu.WBP_PauseMenu_C" _returnvalue))
  (set `self.WBP Pause Menu` _returnvalue_2)
  (bind _returnvalue_3 (`|CreateWidget` "/Game/UI/HUD/WBP_Help.WBP_Help_C" _returnvalue))
  (bind _output_get (set `self.WBP Help` _returnvalue_3))
  (`UserWidget.AddToViewport` _output_get 0))

(event `Pause Game`
  (bind _returnvalue (`self.GetOwningPlayerController`))
  (bind _wbp_pause_menu (`self.WBP Pause Menu`))
  ;[0 0 0] Pause Game Function
  (`UserWidget.AddToViewport` _wbp_pause_menu 0)
  (set `PlayerController.bShowMouseCursor` true _returnvalue)
  (`WidgetBlueprintLibrary.SetInputMode_GameAndUIEx` _returnvalue _wbp_pause_menu))

(event `Toggle Controls`
  ;[0 0 0] Toggle Controls Function
  (bind _isa (`/Engine/EditorBlueprintResources/StandardMacros.FlipFlop`)
    (:`A`
      _)
    (:`B`
      _))
  (set `/Game/UI/HUD/WBP_Help.Show Controls` _isa (`self.WBP Help`)))

(event `Show Interact Hint`
  (params (`Show Interact Hint` :type Boolean))
  ;[0 0 0] Show Interact Hint Function
  (set `/Game/UI/HUD/WBP_Help.Show Interact Hint` `Show Interact Hint` (`self.WBP Help`)))

(event `Show Get Up Hint`
  (params (`Show Get Up Hint` :type Boolean))
  ;[0 0 0] Show Get Up Hint Function
  (set `/Game/UI/HUD/WBP_Help.Show Get Up Hint` `Show Get Up Hint` (`self.WBP Help`)))

(event `self.ReceiveDrawHUD`
  (params (SizeX :type Integer) (SizeY :type Integer))
  (bind _asbp_lobby_player_state (cast `/Game/Blueprints/Lobby/BP_LobbyPlayerState` (`GameplayStatics.GetPlayerState` 0)))
  (`self.DrawText` (`PlayerState.GetPlayerName` _asbp_lobby_player_state) (struct :`A` 1) 0.0 0.0 null))

(fn `Open Player Change UI`
  (params (`Player Controller` :type "/Game/Blueprints/Lobby/BP_LobbyPlayerController Object Reference"))
  (bind _returnvalue (`self.GetOwningPlayerController`))
  (bind _wbp_player_change (`self.WBP Player Change`))
  (`/Engine/EditorBlueprintResources/StandardMacros.IsValid` (`self.WBP Player Change`)
    (:`Is Valid`
      _)
    (:`Is Not Valid`
      (bind _returnvalue_2 (`|CreateWidget` "/Game/UI/CharacterCustomization/WBP_PlayerColorChange.WBP_PlayerColorChange_C" null `Player Controller`))
      (set `self.WBP Player Change` _returnvalue_2)))
  (`UserWidget.AddToViewport` _wbp_player_change 0)
  (set `PlayerController.bShowMouseCursor` true _returnvalue)
  (`WidgetBlueprintLibrary.SetInputMode_UIOnlyEx` _returnvalue _wbp_player_change)
  (bind _player_image_ref (`/Game/Blueprints/Characters/BP_LobbyCharacter.Set Player View UI` (cast `/Game/Blueprints/Characters/BP_LobbyCharacter` (`self.GetOwningPawn`) :!pure true)))
  (set `/Game/UI/CharacterCustomization/WBP_PlayerColorChange.Player Image Ref` _player_image_ref (`self.WBP Player Change`)))

(fn `UserConstructionScript`)