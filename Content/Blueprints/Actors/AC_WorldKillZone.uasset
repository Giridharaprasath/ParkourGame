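; AC_WorldKillZone is a world kill zone that catches lobby characters hitting its box.
; On a component hit, it casts the other actor to BP_LobbyCharacter, ends its ragdoll and calls FreeFall with a destination location, rather than killing it.
; The construction script sets the box's world transform from Height and Size variables, forming a wide slab with fixed vertical scale.
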(event `self.Box.OnComponentHit`
  (params (HitComponent :type "PrimitiveComponent Object Reference") (OtherActor :type "Actor Object Reference") (OtherComp :type "PrimitiveComponent Object Reference") (NormalImpulse :type "Vector Structure") (Hit :type "HitResult Structure (by ref)"))
  (bind _asbp_lobby_character (cast `/Game/Blueprints/Characters/BP_LobbyCharacter` OtherActor))
  (`ALSBaseCharacter.RagdollEnd` _asbp_lobby_character)
  (`/Game/Blueprints/Characters/BP_LobbyCharacter.Free Fall` _asbp_lobby_character (`self.Dest Location`)))

(fn `UserConstructionScript`
  (bind _size (`self.Size`))
  (`SceneComponent.K2_SetWorldTransform` (`self.Box`) (`KismetMathLibrary.MakeTransform` (`KismetMathLibrary.MakeVector` 0.0 0.0 (`self.Height`)) (struct) (`KismetMathLibrary.MakeVector` _size _size 2.0)) false false))