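; Lobby actor that marks a zone where a player character can change its color.
; A box trigger casts overlapping actors to BP_LobbyCharacter and calls ChangePlayerColor with true on entering and false on leaving, printing a debug message each time.
; The construction script applies M_Tiles to the static mesh and tints both top colors the same light blue.
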(event `self.Box.OnComponentBeginOverlap`
  (params (OverlappedComponent :type "PrimitiveComponent Object Reference") (OtherActor :type "Actor Object Reference") (OtherComp :type "PrimitiveComponent Object Reference") (OtherBodyIndex :type Integer) (bFromSweep :type Boolean) (SweepResult :type "HitResult Structure (by ref)"))
  (bind _asbp_lobby_character (cast `/Game/Blueprints/Characters/BP_LobbyCharacter` OtherActor))
  (`/Game/Blueprints/Characters/BP_LobbyCharacter.Change Player Color` _asbp_lobby_character true)
  (`KismetSystemLibrary.PrintString` "Can Change Player Color"))

(event `self.Box.OnComponentEndOverlap`
  (params (OverlappedComponent :type "PrimitiveComponent Object Reference") (OtherActor :type "Actor Object Reference") (OtherComp :type "PrimitiveComponent Object Reference") (OtherBodyIndex :type Integer))
  (bind _asbp_lobby_character (cast `/Game/Blueprints/Characters/BP_LobbyCharacter` OtherActor))
  (`/Game/Blueprints/Characters/BP_LobbyCharacter.Change Player Color` _asbp_lobby_character false)
  (`KismetSystemLibrary.PrintString` "Can't Change Player Color"))

(fn `UserConstructionScript`
  (`PrimitiveComponent.SetMaterial` (`self.StaticMesh`) 0 "/ALSV4_CPP/AdvancedLocomotionV4/Environment/Materials/M_Tiles.M_Tiles")
  (`MeshComponent.SetVectorParameterValueOnMaterials` (`self.StaticMesh`) "TopColor_1" (0.18 0.6 0.9))
  (`MeshComponent.SetVectorParameterValueOnMaterials` (`self.StaticMesh`) "TopColor_2" (0.18 0.6 0.9)))