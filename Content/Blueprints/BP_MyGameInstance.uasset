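; Game instance that manages multiplayer sessions and persists player color through a save game.
; Advanced Sessions nodes host a listen server on the open world level, find, join (including via invites) or cancel searches, showing a loading screen during transitions.
; Network and travel errors route to QuitToMenu, which destroys the session and opens the main menu.
; Init loads or creates the save slot, and color changes save immediately.
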(event `self.ReceiveInit`
  ;[0 0 0] Init Function
  (`self.Check Save Game`))

(event `self.HandleNetworkError`
  (params (FailureType :type "ENetworkFailure Enum" :default "NetDriverAlreadyExists") (bIsServer :type Boolean))
  ;[0 0 0] Quit due to Network Error Function
  (`KismetSystemLibrary.PrintString` (`|GetEnumeratorNameAsString` FailureType))
  (`self.Quit To Menu` (`self.Player Controller`)))

(event `Show Loading Screen`
  ;[0 0 0] Show Loading Screen Function
  (`/Engine/EditorBlueprintResources/StandardMacros.IsValid` (`self.WBP Loading Screen`)
    (:`Is Valid`
      _)
    (:`Is Not Valid`
      (bind _returnvalue (`|CreateWidget` "/Game/UI/WBP_LoadingScreen.WBP_LoadingScreen_C" (`self.Player Controller`)))
      (set `self.WBP Loading Screen` _returnvalue)))
  (`UserWidget.AddToViewport` (`self.WBP Loading Screen`) 0))

(event `self.HandleTravelError`
  (params (FailureType :type "ETravelFailure Enum" :default "NoLevel"))
  ;[0 0 0] Quit due to Travel Error Function
  (`KismetSystemLibrary.PrintString` (`|GetEnumeratorNameAsString` FailureType))
  (`self.Quit To Menu` (`self.Player Controller`)))

(event `Cancel Find Sessions`
  (params (`Player Controller` :type "PlayerController Object Reference"))
  ;[0 0 0] Cancel Find Sessions Function
  (`CancelFindSessionsCallbackProxy.CancelFindSessions` `Player Controller`
    (:`OnSuccess`
      (`KismetSystemLibrary.PrintString` "Stopped Searching!!"))))

(event `Quit To Menu`
  (params (`Player Controller` :type "PlayerController Object Reference"))
  ;[0 0 0] Quit To Menu / Destroy Session Function
  (`self.Show Loading Screen`)
  (`DestroySessionCallbackProxy.DestroySession` `Player Controller`
    (:`OnSuccess`
      _)
    (:`OnFailure`
      _))
  (`GameplayStatics.OpenLevelBySoftObjectPtr` "/Game/Maps/MainMenu_Level.MainMenu_Level")
  (`KismetSystemLibrary.PrintString` "Leaving Session")
  (`Widget.RemoveFromParent` (`self.WBP Loading Screen`)))

(event `Host Session`
  (params (PlayerController :type "PlayerController Object Reference") (`Sesssion Settings` :type "/Game/Blueprints/Structures/F_SessionSettings Structure"))
  ;[0 0 0] Host Session Function
  (bind _output_get (set `self.Player Controller` PlayerController))
  (`self.Show Loading Screen`)
  (`CreateSessionCallbackProxyAdvanced.CreateAdvancedSession` (`.SessionSettings_4_3CBF06A6483C7E31F813A0AD414EACC7` (break `/Game/Blueprints/Structures/F_SessionSettings` `Sesssion Settings`)) _output_get 100 0 (`self.Use LAN`)
    (:`OnSuccess`
      (set `self.Session Settings` `Sesssion Settings`)
      (`GameplayStatics.OpenLevelBySoftObjectPtr` "/Game/Maps/OpenWorld_Level.OpenWorld_Level" true "?listen")
      (`KismetSystemLibrary.PrintString` "Session Created"))
    (:`OnFailure`
      (`KismetSystemLibrary.PrintString` "Cant Start Session" true true (struct :`G` 0.66 :`B` 1.0 :`A` 1.0) 10.0)
      (`Widget.RemoveFromParent` (`self.WBP Loading Screen`)))))

(event `Join Session`
  (params (`Player Controller` :type "PlayerController Object Reference") (`Search Result` :type "BlueprintSessionResult Structure"))
  ;[0 0 0] Join Session Function
  (bind _output_get (set `self.Player Controller` `Player Controller`))
  (`self.Show Loading Screen`)
  (`JoinSessionCallbackProxy.JoinSession` _output_get `Search Result`
    (:`OnSuccess`
      (`KismetSystemLibrary.PrintString` "Session Joined"))
    (:`OnFailure`
      (`KismetSystemLibrary.PrintString` "Cant Join Session" true true (struct :`G` 0.66 :`B` 1.0 :`A` 1.0) 10.0)
      (`Widget.RemoveFromParent` (`self.WBP Loading Screen`)))))

(event `Find Sessions`
  (params (`Player Controller` :type "PlayerController Object Reference"))
  ;[0 0 0] Find Sessions Function
  (bind _results (`FindSessionsCallbackProxyAdvanced.FindSessionsAdvanced` `Player Controller` 50 (`self.Use LAN`) "AllServers")
    (:`OnSuccess`
      _)
    (:`OnFailure`
      _))
  (`self.Sessions Found` _results))

(event `self.OnSessionInviteAccepted`
  (params (LocalPlayerNum :type Integer) (PersonInvited :type "BPUniqueNetId Structure") (SessionToJoin :type "BlueprintSessionResult Structure (by ref)"))
  ;[0 0 0] Join Session via Steam Invite Function
  (`self.Show Loading Screen`)
  (bind _output_get (set `self.Player Controller` (`GameplayStatics.GetPlayerController` 0)))
  (`self.Join Session` _output_get SessionToJoin))

(event `Set Player Info`
  (params (`Player Info` :type "/Game/Blueprints/Structures/F_PlayerInfo Structure"))
  ;[0 0 0] Set Player Info Function
  (set `self.Player Info` `Player Info`))

(event `Set Player Color`
  (params (`Player Color` :type "/Game/Blueprints/Structures/F_PlayerColor Structure"))
  ;[0 0 0] Set Player Color Function
  (set `self.Player Color` `Player Color`)
  (`self.Save Game`))

(fn `Check Save Game`
  (bind _returnvalue (`GameplayStatics.DoesSaveGameExist` (`self.Save Game Name`)))
  (if _returnvalue
    (`KismetSystemLibrary.PrintString` "Save Game Exists" true true (struct :`G` 0.66 :`B` 1.0 :`A` 1.0) 5.0)
    (`self.Load Game`)
    (`self.Save Game`)
    (else
      (`KismetSystemLibrary.PrintString` "Save Game Doesn't Exists" true true (struct :`G` 0.66 :`B` 1.0 :`A` 1.0) 5.0)
      (`self.Save Game`))))

(fn `Delete Save Game`
  (`GameplayStatics.DeleteGameInSlot` (`self.Save Game Name`)))

(fn `Load Game`
  (bind _returnvalue (`GameplayStatics.LoadGameFromSlot` (`self.Save Game Name`)))
  (bind _asbp_my_save_game (cast `/Game/Blueprints/BP_MySaveGame` _returnvalue))
  (bind _output_get (set `self.BP My Save Game` _asbp_my_save_game))
  (set `self.Player Color` (`/Game/Blueprints/BP_MySaveGame.Player Color` _output_get))
  (`KismetSystemLibrary.PrintString` "Save Game Loaded" true true (struct :`G` 0.66 :`B` 1.0 :`A` 1.0) 5.0))

(fn `Save Game`
  (bind _bp_my_save_game (`self.BP My Save Game`))
  (`/Engine/EditorBlueprintResources/StandardMacros.IsValid` (`self.BP My Save Game`)
    (:`Is Valid`
      _)
    (:`Is Not Valid`
      (bind _returnvalue (`GameplayStatics.CreateSaveGameObject` "/Game/Blueprints/BP_MySaveGame.BP_MySaveGame_C"))
      (set `self.BP My Save Game` _returnvalue)))
  (set `/Game/Blueprints/BP_MySaveGame.Player Color` (`self.Player Color`) _bp_my_save_game)
  (`GameplayStatics.SaveGameToSlot` _bp_my_save_game (`self.Save Game Name`))
  (`KismetSystemLibrary.PrintString` "Game Saved" true true (struct :`G` 0.66 :`B` 1.0 :`A` 1.0) 5.0))